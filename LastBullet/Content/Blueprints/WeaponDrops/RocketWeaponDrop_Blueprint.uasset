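; Rocket weapon pickup that gives the first-person character a weapon on overlap and respawns after a short delay.
; While shown, the Drop component spins each tick.
; A box overlap by the character hides Drop, toggles the Luz component's visibility, calls PickWeapon and starts a timer.
; The timer runs spawnDrop to show Drop and toggle Luz again, with Drop's hidden state gating both spin and pickup.
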(event `self.ReceiveTick`
  (params (DeltaSeconds :type "Float (single-precision)"))
  (if (not (`SceneComponent.bHiddenInGame` (`self.Drop`)))
    (`SceneComponent.K2_AddLocalRotation` (`self.Drop`) (struct :`Pitch` 1.0) false false)))

(event `self.Box.OnComponentBeginOverlap`
  (params (OverlappedComponent :type "PrimitiveComponent Object Reference") (OtherActor :type "Actor Object Reference") (OtherComp :type "PrimitiveComponent Object Reference") (OtherBodyIndex :type Integer) (bFromSweep :type Boolean) (SweepResult :type "HitResult Structure (by ref)"))
  (if (not (`SceneComponent.bHiddenInGame` (`self.Drop`)))
    (bind _asfirst_person_character (cast `/Game/FirstPersonBP/Blueprints/FirstPersonCharacter` OtherActor))
    (`SceneComponent.SetHiddenInGame` (`self.Drop`) true false)
    (`SceneComponent.ToggleVisibility` (`self.Luz`) false)
    (`/Game/FirstPersonBP/Blueprints/FirstPersonCharacter.Pick Weapon` _asfirst_person_character "NewEnumerator2")
    (`KismetSystemLibrary.K2_SetTimer` null "spawnDrop" 5.0)))

(fn `spawnDrop`
  (`SceneComponent.SetHiddenInGame` (`self.Drop`) false false)
  (`SceneComponent.ToggleVisibility` (`self.Luz`) false))

(fn `UserConstructionScript`)